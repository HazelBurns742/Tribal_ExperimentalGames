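; Game instance that sets up the server-side turn managers for a multiplayer turn-based session and registers joining clients.
; On Init or LevelOpened, the server spawns TurnManager and TurnManagerBp with delays between, stores both references and broadcasts the Blueprint manager's spawn.
; RunOnSever passes the client count to that manager, creates the player's widget and adds the client to the session.
; The owner-controller polling timer and both event bindings are disconnected.
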(event Custom|LevelOpened
  ;[0 0 0] When server jois, spawn actor/scripts in scene
  (if (Networking|IsServer)
    (bind _returnvalue (Game|SpawnActorfromClass "/Script/Tribal_Experimental.TurnManager" (Math|Conversions|ToTransform(Vector) (Math|Vector|VectorZero)) "AlwaysSpawn" "MultiplyWithRoot" (Game|GetPlayerController 0) 0))
    (Utilities|FlowControl|Delay 2.0)
    (Variables|Default|SetTurnManager _returnvalue)
    (bind _returnvalue_2 (Game|SpawnActorfromClass "/Game/Blueprints/TurnManagerBp.TurnManagerBp_C" (Math|Conversions|ToTransform(Vector) (Math|Vector|VectorZero)) "AlwaysSpawn" "MultiplyWithRoot" (Variables|Default|GetOwnerController) 0))
    (Utilities|FlowControl|Delay 2.0)
    (Variables|Default|SetTurnManagerBPRef _returnvalue_2)
    (Default|CallTurnManagerBpSpawned)))

(event Custom|RunOnSever
  (bind _turnmanagerbpref (Variables|Default|GetTurnManagerBPRef))
  ;[0 0 0] When client joins, call functions
  (Development|PrintString "CIENT JOIN!?" true true "(R=0.318574,G=0.000000,B=1.000000,A=1.000000)")
  (Utilities|IsValid _turnmanagerbpref
    (:Is%20Valid
      (Development|PrintString "REF VALID!!" true true "(R=0.318574,G=0.000000,B=1.000000,A=1.000000)")
      (bind _output_get (Variables|/Script/Tribal_Experimental.TurnManager|SetClientNum _turnmanagerbpref (Variables|Default|GetNumOfClients)))
      (Development|PrintString "Called add client" true true "(R=0.318574,G=0.000000,B=1.000000,A=1.000000)")
      (Class|TurnManager|CreateandAddWidgettoViewport _turnmanagerbpref (Game|GetPlayerController (- _output_get 1)))
      (Development|PrintString "Called create and add widget, for player" true true "(R=0.318574,G=0.000000,B=1.000000,A=1.000000)")
      (Development|PrintString (Utilities|GetDisplayName (Game|GetPlayerController (- _output_get 1))))
      (Class|TurnManager|AddClienttoSession _turnmanagerbpref)
      (Development|PrintString "Called add client to session" true true "(R=0.318574,G=0.000000,B=1.000000,A=1.000000)"))))

(event Custom|OwnerFound?
  (Utilities|IsValid (Variables|Default|GetOwnerController)))

(event EventInit
  ;[0 0 0] When server jois, spawn actor/scripts in scene
  (if (Networking|IsServer)
    (bind _returnvalue (Game|SpawnActorfromClass "/Script/Tribal_Experimental.TurnManager" (Math|Conversions|ToTransform(Vector) (Math|Vector|VectorZero)) "AlwaysSpawn" "MultiplyWithRoot" (Game|GetPlayerController 0) 0))
    (Utilities|FlowControl|Delay 2.0)
    (Variables|Default|SetTurnManager _returnvalue)
    (bind _returnvalue_2 (Game|SpawnActorfromClass "/Game/Blueprints/TurnManagerBp.TurnManagerBp_C" (Math|Conversions|ToTransform(Vector) (Math|Vector|VectorZero)) "AlwaysSpawn" "MultiplyWithRoot" (Variables|Default|GetOwnerController) 0))
    (Utilities|FlowControl|Delay 2.0)
    (Variables|Default|SetTurnManagerBPRef _returnvalue_2)
    (Default|CallTurnManagerBpSpawned)))

(fn IsPlayerControllerValid
  (bind _returnvalue (Game|GetPlayerController 0))
  (if (Utilities|IsValid _returnvalue)
    (Variables|Default|SetOwnerController _returnvalue)
    (Default|CallOwnerFound)
    (Utilities|Time|ClearTimerbyFunctionName 0 "IsPlayerControllerValid")))

(fn SetTurnManagerBPRef
  (params (TurnManagerBPRef :type Turn%20Manager%20Bp%20Object%20Reference))
  (Variables|Default|SetTurnManagerBPRef TurnManagerBPRef)
  (Default|CallTurnManagerBpSpawned))